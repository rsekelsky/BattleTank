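; Player-controllable tank Blueprint that wires input to driving, aiming, firing and camera switching.
; On BeginPlay it hands the tracks to a movement component and the barrel and turret to an aiming component, and links itself to its health bar widget.
; Axis inputs feed movement intents and rotate an azimuth gimbal and spring arm, while a button toggles between first- and third-person cameras.
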(event EventBeginPlay
  (Class|TankMovementComponent|Initialize (Variables|Default|GetTankMovement) (Variables|Default|GetLeft%20Track) (Variables|Default|GetRight%20Track))
  (Class|TankAimingComponent|Initialize (Variables|Default|GetTankAiming) (Variables|Default|GetBarrel) (Variables|Default|GetTurret))
  (CallFunction|InitializeHealthBarWidget))

(event Input|ActionEvents|InputActionFire
  (params (Key :type Key%20Structure))
  ;[1 1 1] Aim/Fire Input Binding
  (:Pressed
    (Class|Tank|Fire)))

(event Input|ActionEvents|InputActionSwapCamera
  (params (Key :type Key%20Structure))
  ;[1 1 1] Perspective Binding
  (:Pressed
    (Components|Activation|ToggleActive (Variables|Default|GetCamera%20%281P%29))
    (Components|Activation|ToggleActive (Variables|Default|GetCamera%20%283P%29))))

(event Input|AxisEvents|InputAxisMoveForward
  (params (AxisValue :type Float%20%28single-precision%29))
  ;[1 1 1] Movement Input Binding
  (Class|TankMovementComponent|IntendMoveForward (Variables|Default|GetTankMovement) AxisValue))

(event Input|AxisEvents|InputAxisTurnRight
  (params (AxisValue :type Float%20%28single-precision%29))
  ;[1 1 1] Movement Input Binding
  (Class|TankMovementComponent|IntendTurnRight (Variables|Default|GetTankMovement) AxisValue))

(event Input|AxisEvents|InputAxisAimElevation
  (params (AxisValue :type Float%20%28single-precision%29))
  ;[1 1 1] Aim/Fire Input Binding
  (Transformation|AddLocalRotation (Variables|Default|GetSpringArm) (Math|Rotator|MakeRotator 0.0 (* AxisValue 3.0) 0.0) false false))

(event Input|AxisEvents|InputAxisAimAzimuth
  (params (AxisValue :type Float%20%28single-precision%29))
  ;[1 1 1] Aim/Fire Input Binding
  (Transformation|AddLocalRotation (Variables|Default|GetAzimuth%20Gimbal) (Math|Rotator|MakeRotator 0.0 0.0 (* AxisValue 3.0)) false false))

(fn ConstructionScript)

(fn InitializeHealthBarWidget
  (bind _ashealth_bar_bp (Utilities|Casting|CastToHealthBar_BP (UserInterface|GetUserWidgetObject (Variables|Default|GetHealth%20Bar))))
  (Variables|/Game/UI/HealthBar_BP.HealthBar_BP_C|SetBP%20Tank%20Reference _ashealth_bar_bp self)
  (return))